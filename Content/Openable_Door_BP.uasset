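; Openable door actor that swings open and closed with a lock sound.
; OnOpen and OnClose events from its OpenDoor member play or reverse the DoorSwing timeline.
; The timeline's OpenAngle track drives yaw, combined with the rotation cached at BeginPlay so the swing is relative to the door's placement.
; A Sound Timing event track plays the Doorlock sound at the actor's location.
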(event OnOpen(OpenDoor)
  ;[1 1 1] Open/Close Door
  (bind _openangle (Timeline|Door%20Swing Play)
    (:Update
      (Transformation|SetActorRotation (Math|Rotator|CombineRotators (Math|Rotator|MakeRotator 0.0 0.0 _openangle) (Variables|Default|GetInitialRotation))))
    (:Sound%20Timing
      (Audio|PlaySoundatLocation "/Game/door-lock.door-lock" (Transformation|GetActorLocation) "0, 0, 0" 1.0 1.0 0.0 0 0 0))))

(event OnClose(OpenDoor)
  ;[1 1 1] Open/Close Door
  (bind _openangle (Timeline|Door%20Swing Reverse)
    (:Update
      (Transformation|SetActorRotation (Math|Rotator|CombineRotators (Math|Rotator|MakeRotator 0.0 0.0 _openangle) (Variables|Default|GetInitialRotation))))
    (:Sound%20Timing
      (Audio|PlaySoundatLocation "/Game/door-lock.door-lock" (Transformation|GetActorLocation) "0, 0, 0" 1.0 1.0 0.0 0 0 0))))

(event EventBeginPlay
  ;[1 1 1] Setup Rotation
  (Variables|Default|SetInitialRotation (Transformation|GetActorRotation)))

(fn ConstructionScript)